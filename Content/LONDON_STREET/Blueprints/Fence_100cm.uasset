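; Spline-driven fence builder for the London Street content, laying repeated fence segments along an editable spline.
; The construction script divides the spline length by Spacing and adds a spline mesh component for each interval, with query and physics collision.
; Each segment takes world-space start and end points from the spline, with tangents from spline direction times TangentScale.
; The event graph holds no active logic.
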(fn `UserConstructionScript`
  (bind _spline (`self.Spline`))
  (bind _tangent_scale (`self.tangent scale`))
  (bind _spacing (`self.Spacing`))
  (for _index (range (+ (`.ReturnValue` (`KismetMathLibrary.FMod` (`SplineComponent.GetSplineLength` (`self.Spline`)) _spacing)) 1))
    (bind _returnvalue (`AddComponent|NODE_AddSplineMeshComponent-8` :`bManualAttachment` true))
    (`PrimitiveComponent.SetCollisionEnabled` _returnvalue "QueryAndPhysics")
    (bind _returnvalue_2 (* _index _spacing))
    (bind _returnvalue_3 (+ _returnvalue_2 _spacing))
    (`SplineMeshComponent.SetStartAndEnd` _returnvalue (`SplineComponent.GetLocationAtDistanceAlongSpline` _spline _returnvalue_2 "World") (* (`SplineComponent.GetDirectionAtDistanceAlongSpline` _spline _returnvalue_2 "World") _tangent_scale) (`SplineComponent.GetLocationAtDistanceAlongSpline` _spline _returnvalue_3 "World") (* (`SplineComponent.GetDirectionAtDistanceAlongSpline` _spline _returnvalue_3 "World") _tangent_scale) true)))