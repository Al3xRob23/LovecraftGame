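; Spline-driven street builder actor that lays road or pavement pieces along a spline in London Street.
; The construction script adds one spline mesh with collision per Spacing interval, using world-space positions and scaled directions as tangents.
; The Pavement flag selects curb meshes, with PavementRight choosing the side, and applies cobble and fence-cap materials.
; Otherwise segments keep the component template's mesh; the event graph is unused.
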(fn `UserConstructionScript`
  (bind _spline (`self.Spline`))
  (bind _tangent_scale (`self.tangent scale`))
  (bind _spline_2 (`self.Spline`))
  (bind _tangent_scale_2 (`self.tangent scale`))
  (bind _spline_3 (`self.Spline`))
  (bind _spline_4 (`self.Spline`))
  (bind _tangent_scale_3 (`self.tangent scale`))
  (bind _spacing (`self.Spacing`))
  (for _index (range (+ (`.ReturnValue` (`KismetMathLibrary.FMod` (`SplineComponent.GetSplineLength` (`self.Spline`)) _spacing)) 1))
    (if (`self.Pavement`)
      (bind _returnvalue (`AddComponent|NODE_AddSplineMeshComponent-5` :`bManualAttachment` true))
      (if (`self.Pavement_Right`)
        (`PrimitiveComponent.SetCollisionEnabled` _returnvalue "QueryAndPhysics")
        (`StaticMeshComponent.SetStaticMesh` _returnvalue "/Game/LONDON_STREET/Meshes/Road/pavement_straight_element_curb_right.pavement_straight_element_curb_right")
        (`PrimitiveComponent.SetMaterial` _returnvalue 0 "/Game/LONDON_STREET/Materials/Cobble.Cobble")
        (`PrimitiveComponent.SetMaterial` _returnvalue 1 "/Game/LONDON_STREET/Materials/Fence_Cap.Fence_Cap")
        (`SceneComponent.K2_AttachToComponent` _spline (`self.Scene`) "None" "KeepRelative" "KeepRelative" "KeepRelative" true)
        (bind _returnvalue_2 (* _index _spacing))
        (bind _returnvalue_3 (+ _returnvalue_2 _spacing))
        (`SplineMeshComponent.SetStartAndEnd` _returnvalue (`SplineComponent.GetLocationAtDistanceAlongSpline` _spline_3 _returnvalue_2 "World") (* (`SplineComponent.GetDirectionAtDistanceAlongSpline` _spline_3 _returnvalue_2 "World") _tangent_scale) (`SplineComponent.GetLocationAtDistanceAlongSpline` _spline_3 _returnvalue_3 "World") (* (`SplineComponent.GetDirectionAtDistanceAlongSpline` _spline_3 _returnvalue_3 "World") _tangent_scale) true)
        (else
          (`PrimitiveComponent.SetCollisionEnabled` _returnvalue "QueryAndPhysics")
          (`StaticMeshComponent.SetStaticMesh` _returnvalue "/Game/LONDON_STREET/Meshes/Road/pavement_straight_element_curb.pavement_straight_element_curb")
          (`PrimitiveComponent.SetMaterial` _returnvalue 0 "/Game/LONDON_STREET/Materials/Cobble.Cobble")
          (`PrimitiveComponent.SetMaterial` _returnvalue 1 "/Game/LONDON_STREET/Materials/Fence_Cap.Fence_Cap")
          (`SceneComponent.K2_AttachToComponent` _spline (`self.Scene`) "None" "KeepRelative" "KeepRelative" "KeepRelative" true)
          (`SplineMeshComponent.SetStartAndEnd` _returnvalue (`SplineComponent.GetLocationAtDistanceAlongSpline` _spline_2 _returnvalue_2 "World") (* (`SplineComponent.GetDirectionAtDistanceAlongSpline` _spline_2 _returnvalue_2 "World") _tangent_scale_2) (`SplineComponent.GetLocationAtDistanceAlongSpline` _spline_2 _returnvalue_3 "World") (* (`SplineComponent.GetDirectionAtDistanceAlongSpline` _spline_2 _returnvalue_3 "World") _tangent_scale_2) true)))
      (else
        (bind _returnvalue_4 (`AddComponent|NODE_AddSplineMeshComponent-6` :`bManualAttachment` true))
        (`PrimitiveComponent.SetCollisionEnabled` _returnvalue_4 "QueryAndPhysics")
        (`SceneComponent.K2_AttachToComponent` _spline (`self.Scene`) "None" "KeepRelative" "KeepRelative" "KeepRelative" true)
        (`SplineMeshComponent.SetStartAndEnd` _returnvalue_4 (`SplineComponent.GetLocationAtDistanceAlongSpline` _spline_4 _returnvalue_2 "World") (* (`SplineComponent.GetDirectionAtDistanceAlongSpline` _spline_4 _returnvalue_2 "World") _tangent_scale_3) (`SplineComponent.GetLocationAtDistanceAlongSpline` _spline_4 _returnvalue_3 "World") (* (`SplineComponent.GetDirectionAtDistanceAlongSpline` _spline_4 _returnvalue_3 "World") _tangent_scale_3) true)))))