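; Configurable shop-front prop for the London Street environment, with variants for the sign and showcase.
; The Construction Script reads option variables to swap static meshes for the large sign, showcases and showcase glass.
; The Showcase option runs last, clearing ShowcaseTall, toggling Showcase3's visibility and setting the Showcase4 and glass meshes.
; The Event Graph holds only unused default events, so there is no runtime logic.
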(fn `UserConstructionScript`
  (if (`self.Shop_Sign_Large`)
    (`StaticMeshComponent.SetStaticMesh` (`self.Shop_Sign Large`) "/Game/LONDON_STREET/Meshes/Facade/shop_sign_large_2.shop_sign_large_2"))
  (if (`self.Showcase_tall`)
    (`StaticMeshComponent.SetStaticMesh` (`self.Showcase_3`) "/Game/LONDON_STREET/Meshes/Facade/shop_showcase_3.shop_showcase_3")
    (`StaticMeshComponent.SetStaticMesh` (`self.Glass`) "/Game/LONDON_STREET/Meshes/Facade/glass_showcase2.glass_showcase2"))
  (if (`self.Showcase`)
    (set `self.Showcase_tall` false)
    (`SceneComponent.ToggleVisibility` (`self.Showcase_3`) false)
    (`StaticMeshComponent.SetStaticMesh` (`self.Showcase_4`) "/Game/LONDON_STREET/Meshes/Facade/shop_showcase_4.shop_showcase_4")
    (`StaticMeshComponent.SetStaticMesh` (`self.Glass`) "/Game/LONDON_STREET/Meshes/Facade/glass_showcase2.glass_showcase2")))