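; Font is a London Street actor that displays two configurable pieces of 3D text.
; Its construction script applies Text1 and TextColor to TextRender, and Text2 and TextColor2 to TextRender1, converting each linear color with sRGB enabled.
; The event graph holds only disabled placeholder events, so the Blueprint adds no runtime logic.
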(fn `UserConstructionScript`
  (`TextRenderComponent.K2_SetText` (`self.TextRender`) (`self.text1`))
  (`TextRenderComponent.SetTextRenderColor` (`self.TextRender`) (`KismetMathLibrary.Conv_LinearColorToColor` (`self.text color`)))
  (`TextRenderComponent.K2_SetText` (`self.TextRender1`) (`self.text2`))
  (`TextRenderComponent.SetTextRenderColor` (`self.TextRender1`) (`KismetMathLibrary.Conv_LinearColorToColor` (`self.text color_2`))))