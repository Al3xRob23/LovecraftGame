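; Large fence pillar Blueprint for the London street set, with a choice of two post-top cap meshes.
; Its construction script uses the Cap1 and Cap2 flags to assign the matching cap mesh.
; Enabling Cap2 also clears the Cap1 flag and toggles that cap's visibility.
; The event graph holds only disabled placeholder events, so the pillar has no runtime logic.
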(fn `UserConstructionScript`
  (if (`self.Cap_1`)
    (`StaticMeshComponent.SetStaticMesh` (`self.Cap 1`) "/Game/LONDON_STREET/Meshes/Props/fence_post_top.fence_post_top"))
  (if (`self.Cap_2`)
    (set `self.Cap_1` false)
    (`SceneComponent.ToggleVisibility` (`self.Cap 1`) false)
    (`StaticMeshComponent.SetStaticMesh` (`self.Cap 2`) "/Game/LONDON_STREET/Meshes/Props/fence_post_top_2.fence_post_top_2")))