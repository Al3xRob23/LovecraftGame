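; Lantern_Wall_2 is a lantern Blueprint in the London Street content with a configurable point light.
; When the Light flag is set, the construction script toggles the PointLight's visibility, rather than setting it explicitly, and applies the Intensity, Attenuation and Colour variables.
; The event graph holds only disabled placeholder events, so it adds no runtime behavior.
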(fn `UserConstructionScript`
  (if (`self.Light?`)
    (`SceneComponent.ToggleVisibility` (`self.PointLight`) false)
    (`LightComponent.SetIntensity` (`self.PointLight`) (`self.Intensity`))
    (`PointLightComponent.SetAttenuationRadius` (`self.PointLight`) (`self.Attenuation`))
    (`LightComponent.SetLightColor` (`self.PointLight`) (`self.Colour`) true)))