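; Bay window prop for the London street environment, with an optional fake interior and curtains.
; The construction script toggles the visibility of the InteriorFake component when Interior is set, and of six curtain components when Curtains is set.
; Each flag flips the component's default visibility rather than setting it explicitly, without propagating to children.
; The event graph holds only disabled placeholder events, so there is no runtime logic.
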(fn `UserConstructionScript`
  (if (`self.Interior`)
    (`SceneComponent.ToggleVisibility` (`self.Interior_Fake`) false))
  (if (`self.Curtains`)
    (`SceneComponent.ToggleVisibility` (`self.Curtain_1`) false)
    (`SceneComponent.ToggleVisibility` (`self.Curtain_2`) false)
    (`SceneComponent.ToggleVisibility` (`self.Curtain_3`) false)
    (`SceneComponent.ToggleVisibility` (`self.Curtain_4`) false)
    (`SceneComponent.ToggleVisibility` (`self.Curtain_5`) false)
    (`SceneComponent.ToggleVisibility` (`self.Curtain_6`) false)))