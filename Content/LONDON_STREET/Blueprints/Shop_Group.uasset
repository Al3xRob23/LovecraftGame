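; Configurable shop-front actor for the London street set, assembled from sign, shop group, showcase and glass meshes.
; The construction script reads boolean options and assigns the matching static mesh to each component.
; Larger options override earlier ones by clearing their flags and toggling component visibility, with Showcase2 overriding all but the small sign.
; Both showcases share one glass component, and there is no runtime logic.
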(fn `UserConstructionScript`
  (if (`self.Small Sign`)
    (`StaticMeshComponent.SetStaticMesh` (`self.Sign_Small`) "/Game/LONDON_STREET/Meshes/Facade/shop_sign_small.shop_sign_small"))
  (if (`self.Medium Sign`)
    (`StaticMeshComponent.SetStaticMesh` (`self.Sign_Medium_2`) "/Game/LONDON_STREET/Meshes/Facade/shop_sign_medium_2.shop_sign_medium_2"))
  (if (`self.Large Sign`)
    (set `self.Small Sign` false)
    (`SceneComponent.ToggleVisibility` (`self.Sign_Small`) false)
    (set `self.Medium Sign` false)
    (`SceneComponent.ToggleVisibility` (`self.Sign_Medium_2`) false)
    (`StaticMeshComponent.SetStaticMesh` (`self.Sign_Large`) "/Game/LONDON_STREET/Meshes/Facade/shop_sign_large_2.shop_sign_large_2"))
  (if (`self.Shop Group Medium`)
    (`StaticMeshComponent.SetStaticMesh` (`self.Shop_Group_Medium`) "/Game/LONDON_STREET/Meshes/Facade/shop_group_medium.shop_group_medium"))
  (if (`self.Showcase 1`)
    (set `self.Shop Group Medium` false)
    (`SceneComponent.ToggleVisibility` (`self.Shop_Group_Medium`) false)
    (`StaticMeshComponent.SetStaticMesh` (`self.Showcase`) "/Game/LONDON_STREET/Meshes/Facade/shop_showcase.shop_showcase")
    (`StaticMeshComponent.SetStaticMesh` (`self.glass`) "/Game/LONDON_STREET/Meshes/Facade/glass_showcase.glass_showcase"))
  (if (`self.Showcase 2`)
    (set `self.Large Sign` false)
    (`SceneComponent.ToggleVisibility` (`self.Sign_Large`) false)
    (set `self.Medium Sign` false)
    (`SceneComponent.ToggleVisibility` (`self.Sign_Medium_2`) false)
    (set `self.Shop Group Medium` false)
    (`SceneComponent.ToggleVisibility` (`self.Shop_Group_Medium`) false)
    (set `self.Showcase 1` false)
    (`SceneComponent.ToggleVisibility` (`self.Showcase`) false)
    (`StaticMeshComponent.SetStaticMesh` (`self.Showcase_2`) "/Game/LONDON_STREET/Meshes/Facade/shop_showcase_2.shop_showcase_2")
    (`StaticMeshComponent.SetStaticMesh` (`self.glass`) "/Game/LONDON_STREET/Meshes/Facade/glass_showcase.glass_showcase")))