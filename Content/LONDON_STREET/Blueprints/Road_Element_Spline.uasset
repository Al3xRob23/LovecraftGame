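; Spline-driven road element for the London street environment that builds deformed meshes along an editable spline.
; The construction script adds a spline mesh per segment, using the chosen forward axis and the local locations and tangents of adjacent points to bend it along the curve.
; A Pavement flag selects between two otherwise identical branches, each adding its own spline mesh component.
; The event graph has no active logic.
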(fn `UserConstructionScript`
  (bind _scene (`self.Scene`))
  (bind _spline (`self.Spline`))
  (bind _spline_2 (`self.Spline`))
  (for _index (range (+ (- (`SplineComponent.GetNumberOfSplinePoints` (`self.Spline`)) 2) 1))
    (if (`self.Pavement`)
      (bind _returnvalue (`AddComponent|NODE_AddSplineMeshComponent-4`))
      (`SplineMeshComponent.SetForwardAxis` _returnvalue (`self.Forward Axis`) true)
      (`SceneComponent.K2_AttachToComponent` _returnvalue _scene "None" "KeepRelative" "KeepRelative" "KeepRelative" true)
      (bind _returnvalue_2 (+ _index 1))
      (`SplineMeshComponent.SetStartAndEnd` _returnvalue (`SplineComponent.GetLocationAtSplinePoint` _spline_2 _index "Local") (`SplineComponent.GetTangentAtSplinePoint` _spline_2 _index "Local") (`SplineComponent.GetLocationAtSplinePoint` _spline_2 _returnvalue_2 "Local") (`SplineComponent.GetTangentAtSplinePoint` _spline_2 _returnvalue_2 "Local") true)
      (else
        (bind _returnvalue_3 (`AddComponent|NODE_AddSplineMeshComponent-3`))
        (`SplineMeshComponent.SetForwardAxis` _returnvalue_3 (`self.Forward Axis`) true)
        (`SceneComponent.K2_AttachToComponent` _returnvalue_3 _scene "None" "KeepRelative" "KeepRelative" "KeepRelative" true)
        (`SplineMeshComponent.SetStartAndEnd` _returnvalue_3 (`SplineComponent.GetLocationAtSplinePoint` _spline _index "Local") (`SplineComponent.GetTangentAtSplinePoint` _spline _index "Local") (`SplineComponent.GetLocationAtSplinePoint` _spline _returnvalue_2 "Local") (`SplineComponent.GetTangentAtSplinePoint` _spline _returnvalue_2 "Local") true)))))