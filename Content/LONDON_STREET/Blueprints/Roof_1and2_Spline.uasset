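; Spline-driven roof builder for the London Street environment, offering two roof variants along an editable spline.
; The construction script adds one collision-enabled spline mesh per segment, bending it between neighbouring points using their local positions and tangents.
; The Roof2 flag chooses between two otherwise identical branches, each with its own spline mesh component node.
; All work happens at construction, as the event graph has no active logic.
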(fn `UserConstructionScript`
  (bind _spline (`self.Spline`))
  (bind _scene (`self.Scene`))
  (bind _spline_2 (`self.Spline`))
  (bind _spline_3 (`self.Spline`))
  (for _index (range (+ (- (`SplineComponent.GetNumberOfSplinePoints` (`self.Spline`)) 2) 1))
    (if (`self.Roof 2`)
      (bind _returnvalue (`AddComponent|NODE_AddSplineMeshComponent-5`))
      (`PrimitiveComponent.SetCollisionEnabled` _returnvalue "QueryAndPhysics")
      (`SceneComponent.K2_AttachToComponent` _spline _scene "None" "KeepRelative" "KeepRelative" "KeepRelative" true)
      (bind _returnvalue_2 (+ _index 1))
      (`SplineMeshComponent.SetStartAndEnd` _returnvalue (`SplineComponent.GetLocationAtSplinePoint` _spline_3 _index "Local") (`SplineComponent.GetTangentAtSplinePoint` _spline_3 _index "Local") (`SplineComponent.GetLocationAtSplinePoint` _spline_3 _returnvalue_2 "Local") (`SplineComponent.GetTangentAtSplinePoint` _spline_3 _returnvalue_2 "Local") true)
      (else
        (bind _returnvalue_3 (`AddComponent|NODE_AddSplineMeshComponent-6`))
        (`PrimitiveComponent.SetCollisionEnabled` _returnvalue_3 "QueryAndPhysics")
        (`SceneComponent.K2_AttachToComponent` _spline _scene "None" "KeepRelative" "KeepRelative" "KeepRelative" true)
        (bind _returnvalue_4 (+ _index 1))
        (`SplineMeshComponent.SetStartAndEnd` _returnvalue_3 (`SplineComponent.GetLocationAtSplinePoint` _spline_2 _index "Local") (`SplineComponent.GetTangentAtSplinePoint` _spline_2 _index "Local") (`SplineComponent.GetLocationAtSplinePoint` _spline_2 _returnvalue_4 "Local") (`SplineComponent.GetTangentAtSplinePoint` _spline_2 _returnvalue_4 "Local") true)))))